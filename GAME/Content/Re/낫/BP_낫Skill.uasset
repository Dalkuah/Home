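; BP_낫Skill is a thrown scythe projectile that flies out and returns like a boomerang.
; Tick spins its Box and moves it forward, steering by the owner's camera for one second.
; It then homes on player character 0 with interpolation that tightens over time.
; Box overlaps send OKMessage to AttackOK actors, while touching the owner after a half-second arming delay calls 장착낫 to re-equip and destroys the projectile.
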(event `self.Box.OnComponentBeginOverlap`
  (params (OverlappedComponent :type "PrimitiveComponent Object Reference") (OtherActor :type "Actor Object Reference") (OtherComp :type "PrimitiveComponent Object Reference") (OtherBodyIndex :type Integer) (bFromSweep :type Boolean) (SweepResult :type "HitResult Structure (by ref)"))
  (bind _returnvalue (`self.GetOwner`))
  (bind _returnvalue_2 (`self.GetOwner`))
  (if (and (`self.SET`) (== OtherActor _returnvalue))
    (bind _asbp_player_ox (cast `/Game/aaaaa/ThirdPerson/Blueprints/BP_PlayerOX` _returnvalue))
    (`/Engine/EditorBlueprintResources/StandardMacros.IsValid` _asbp_player_ox
      (:`Is Valid`
        (`/Game/aaaaa/ThirdPerson/Blueprints/BP_PlayerOX.장착:낫` _asbp_player_ox)
        (`self.K2_DestroyActor`)))
    (elif (`KismetSystemLibrary.DoesImplementInterface` OtherActor "/Game/MyGame/AI/AttackOK.AttackOK_C")
      (`/Engine/EditorBlueprintResources/StandardMacros.IsValid` _returnvalue_2
        (:`Is Valid`
          (message `/Game/MyGame/AI/AttackOK.OK!` OtherActor _returnvalue_2))))))

(event `self.ReceiveBeginPlay`
  (set `self.HomingTarget` (`GameplayStatics.GetPlayerCharacter` 0))
  (`KismetSystemLibrary.Delay` 0.5)
  (set `self.SET` true))

(event `self.ReceiveTick`
  (params (DeltaSeconds :type "Float (single-precision)"))
  (bind _totalsec (`self.TotalSec`))
  (set `self.TotalSec` (+ (`self.TotalSec`) DeltaSeconds))
  (`|ExecutionSequence`
    (:`then_0`
      (`SceneComponent.K2_AddRelativeRotation` (`self.Box`) (`KismetMathLibrary.MakeRotator` 0.0 0.0 (* (* DeltaSeconds 360.0) -5.0)) false false)
      (`/Engine/EditorBlueprintResources/StandardMacros.IsValid` (`self.HomingTarget`)
        (:`Is Valid`
          (`self.K2_AddActorWorldOffset` (* (`self.GetActorForwardVector`) (* DeltaSeconds 10000.0)))
          (if (>= _totalsec 1.0)
            (`self.K2_SetActorRotation` (`KismetMathLibrary.RInterpTo` (`self.K2_GetActorRotation`) (`KismetMathLibrary.FindLookAtRotation` (`self.K2_GetActorLocation`) (`self.K2_GetActorLocation` (`self.HomingTarget`))) _totalsec (/ _totalsec 1.0)))
            (else
              (bind _asbp_player_ox (cast `/Game/aaaaa/ThirdPerson/Blueprints/BP_PlayerOX` (`self.GetOwner`)))
              (`self.K2_SetActorRotation` (`SceneComponent.K2_GetComponentRotation` (`/Game/aaaaa/ThirdPerson/Blueprints/BP_PlayerOX.FollowCamera` _asbp_player_ox))))))))))

(fn `UserConstructionScript`)