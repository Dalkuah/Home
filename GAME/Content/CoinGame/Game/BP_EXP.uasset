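; BP_EXP is an experience pickup that adds its ExpValue to the player's BP_PlayerState on overlap, then destroys itself.
; A custom event sets ExpValue, and Tick scales the sphere in proportion to it.
; Within range of the player, Tick homes the actor in by moving it along its forward vector, faster when closer, while smoothly turning it toward the player.
; The physics impulse alternatives are disconnected.
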(event `self.Sphere1.OnComponentBeginOverlap`
  (params (OverlappedComponent :type "PrimitiveComponent Object Reference") (OtherActor :type "Actor Object Reference") (OtherComp :type "PrimitiveComponent Object Reference") (OtherBodyIndex :type Integer) (bFromSweep :type Boolean) (SweepResult :type "HitResult Structure (by ref)"))
  (bind _asbp_player_ox (cast `/Game/aaaaa/ThirdPerson/Blueprints/BP_PlayerOX` OtherActor))
  (bind _asbp_player_state (cast `/Game/CoinGame/GameMode/BP_PlayerState` (`Pawn.PlayerState` _asbp_player_ox)))
  (`/Game/CoinGame/GameMode/BP_PlayerState.AddEXP` _asbp_player_state (`self.Exp Value`))
  (`self.K2_DestroyActor`))

(event `SetExp`
  (params (ExpValue :type Integer)))

(event `/Game/CoinGame/Game/EntityEXP.!!EXP`
  (params (`!!Exp` :type Integer))
  (set `self.Exp Value` `!!Exp`))

(event `self.ReceiveTick`
  (params (DeltaSeconds :type "Float (single-precision)"))
  (bind _returnvalue (`GameplayStatics.GetPlayerCharacter` 0))
  (bind _returnvalue_2 (`self.GetDistanceTo` _returnvalue))
  (`SceneComponent.SetWorldScale3D` (`self.Sphere`) (`KismetMathLibrary.Conv_DoubleToVector` (* (`self.Exp Value`) 0.01)))
  (if (<= _returnvalue_2 2000.0)
    (`self.K2_AddActorWorldOffset` (* (`self.GetActorForwardVector`) (/ (- 10000.0 _returnvalue_2) 2000.0)))
    (`self.K2_SetActorRotation` (`KismetMathLibrary.RInterpTo` (`self.K2_GetActorRotation`) (`KismetMathLibrary.FindLookAtRotation` (`self.K2_GetActorLocation`) (`self.K2_GetActorLocation` _returnvalue)) DeltaSeconds 30.0))))

(event `self.ReceiveBeginPlay`)

(fn `UserConstructionScript`)