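; Spawner actor that creates waves of BP_AI enemies at random offsets and yaws around its Cube component.
; It binds to BP_GameState's state change; Play spawns a wave and starts a looping Spawn2 timer, and Ready clears it.
; Tick rerolls delay and count within configured limits, but the timer keeps the delay sampled when set.
; Each enemy's HP and damage scale with the spawner's accumulated lifetime.
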(event `self.ReceiveBeginPlay`
  (`self.BindGameState`)
  (`KismetSystemLibrary.K2_SetTimer` null "Spawn" 0.0 true))

(event `self.ReceiveTick`
  (params (DeltaSeconds :type "Float (single-precision)"))
  (bind _spawnmaxdelay (`self.SpawnMaxDelay`))
  (bind _spawnmaxrate (`self.SpawnMaxRate`))
  (set `self.TotalSec` (+ (`self.TotalSec`) DeltaSeconds))
  (`|ExecutionSequence`
    (:`then_0`
      (if (== (`self.SpawnMaxDelay`) 0.0)
        (set `self.SpawnDelay` 10.0)
        (else
          (set `self.SpawnDelay` (`KismetMathLibrary.FClamp` (`KismetMathLibrary.RandomFloatInRange` (`self.SpawnMinDelay`) _spawnmaxdelay) 0.0 _spawnmaxdelay)))))
    (:`then_1`
      (if (== (`self.SpawnMaxRate`) 0)
        (set `self.SpawnRate` 3)
        (else
          (set `self.SpawnRate` (`KismetMathLibrary.Clamp` (`KismetMathLibrary.RandomIntegerInRange` (`self.SpawnMinRate`) _spawnmaxrate) 0 _spawnmaxrate)))))))

(fn `BindGameState`
  (bind _asbp_game_state (cast `/Game/CoinGame/GameMode/BP_GameState` (`GameplayStatics.GetGameState`)))
  (add `/Game/CoinGame/GameMode/BP_GameState.EventDispatcher_ChangeGameState` _asbp_game_state (`|CreateDelegate` :!event `Spawn`)))

(fn `Spawn`
  (params (Game :type "/Game/CoinGame/GameMode/EN_GameState Enum" :default "NewEnumerator4"))
  (switch `/Game/CoinGame/GameMode/EN_GameState` Game
    (:`NewEnumerator0`
      (`KismetSystemLibrary.K2_ClearTimer` null "Spawn2"))
    (:`NewEnumerator1`
      (`self.Spawn2`)
      (`KismetSystemLibrary.K2_SetTimer` null "Spawn2" (`self.SpawnDelay`) true))))

(fn `Spawn2`
  (bind _returnvalue (/ (`self.TotalSec`) 5.0))
  (for _ (range 1 (+ (`self.SpawnRate`) 1))
    (bind _returnvalue_2 (`|SpawnActorFromClass` "/Game/MyGame/AI/BP_AI.BP_AI_C" (`KismetMathLibrary.MakeTransform` (+ (`SceneComponent.K2_GetComponentLocation` (`self.Cube`)) (* (`KismetMathLibrary.RandomUnitVector`) (`KismetMathLibrary.RandomFloatInRange` -1000.0 1000.0))) (`KismetMathLibrary.MakeRotator` 0.0 0.0 (+ 0.0 (`KismetMathLibrary.RandomFloatInRange` 0.0 360.0)))) "Undefined" "OverrideRootScale" null null))
    (`/Engine/EditorBlueprintResources/StandardMacros.IsValid` _returnvalue_2
      (:`Is Valid`
        (message `/Game/CoinGame/AISet.AISET` _returnvalue_2 _returnvalue (/ _returnvalue 3.0))))))

(fn `UserConstructionScript`)