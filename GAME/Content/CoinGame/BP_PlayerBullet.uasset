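; BP_PlayerBullet is a physics-driven explosive projectile that damages and knocks back player characters and AI.
; On BeginPlay its Sphere gets a forward impulse with slight random spread, and each tick it rotates to face its velocity.
; Overlaps apply damage through BP_PlayerState or BP_AI, plus knockback along the Arrow.
; Those overlaps or any hit trigger Dead: explosion effects, camera shake, sphere shutdown, then delayed destruction.
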(event `self.ReceiveBeginPlay`
  (`ActorComponent.SetActive` (`self.PlayerSkillFx1`) true false)
  (`PrimitiveComponent.AddImpulse` (`self.Sphere`) (* (`KismetMathLibrary.VLerp` (`KismetMathLibrary.RandomUnitVector`) (`self.GetActorForwardVector`) 0.95) (`self.Power`)) "None" false))

(event `self.Sphere.OnComponentHit`
  (params (HitComponent :type "PrimitiveComponent Object Reference") (OtherActor :type "Actor Object Reference") (OtherComp :type "PrimitiveComponent Object Reference") (NormalImpulse :type "Vector Structure") (Hit :type "HitResult Structure (by ref)"))
  (`self.Dead`))

(event `self.ReceiveTick`
  (params (DeltaSeconds :type "Float (single-precision)"))
  (bind _sphere (`self.Sphere`))
  (`SceneComponent.K2_SetWorldRotation` _sphere (`KismetMathLibrary.Conv_VectorToRotator` (`SceneComponent.GetComponentVelocity` _sphere)) false false))

(event `self.Sphere.OnComponentBeginOverlap`
  (params (OverlappedComponent :type "PrimitiveComponent Object Reference") (OtherActor :type "Actor Object Reference") (OtherComp :type "PrimitiveComponent Object Reference") (OtherBodyIndex :type Integer) (bFromSweep :type Boolean) (SweepResult :type "HitResult Structure (by ref)"))
  (bind _asbp_third_person_character (cast `/Game/aaaaa/ThirdPerson/Blueprints/BP_ThirdPersonCharacter` OtherActor)
    (:`then`
      (bind _asbp_player_state (cast `/Game/CoinGame/GameMode/BP_PlayerState` (`Pawn.PlayerState` _asbp_third_person_character)))
      (`/Game/CoinGame/GameMode/BP_PlayerState.AddDamage` _asbp_player_state 1.0)
      (`CharacterMovementComponent.AddImpulse` (`Character.CharacterMovement` _asbp_third_person_character) (* (`SceneComponent.GetForwardVector` (`self.Arrow`)) 50000.0) false))
    (:`CastFailed`
      (bind _asbp_ai (cast `/Game/MyGame/AI/BP_AI` OtherActor))
      (`/Game/MyGame/AI/BP_AI.AddDamage` _asbp_ai 30.0)
      (`Character.LaunchCharacter` _asbp_ai (* (`SceneComponent.GetForwardVector` (`self.Arrow`)) 5000.0) false false)))
  (`self.Dead`))

(event `Dead`
  (bind _returnvalue (`self.K2_GetActorLocation`))
  (bind _sphere (`self.Sphere`))
  (`ActorComponent.SetActive` (`self.PlayerSkillFx1`) false false)
  (`GameplayStatics.SpawnSoundAtLocation` "/Game/StarterContent/Audio/Explosion_Cue.Explosion_Cue" (`self.K2_GetActorLocation`) (struct) 1.0 1.0 0.0 null null)
  (`GameplayStatics.SpawnEmitterAtLocation` "/Game/StarterContent/Particles/P_Explosion.P_Explosion" _returnvalue (`self.K2_GetActorRotation`) (* (`self.GetActorScale3D`) 1.0))
  (`GameplayStatics.PlayWorldCameraShake` "/Game/CoinGame/BP_CameraShake.BP_CameraShake_C" _returnvalue 0.0 500.0)
  (`PrimitiveComponent.SetSimulatePhysics` _sphere false)
  (`SceneComponent.SetVisibility` _sphere false false)
  (`PrimitiveComponent.SetCollisionEnabled` _sphere "NoCollision")
  (`KismetSystemLibrary.Delay` 2.0)
  (`self.K2_DestroyActor`))

(fn `AddRotation`
  (`SceneComponent.K2_AddLocalRotation` (`self.Sphere`) (struct :`Yaw` 1.0) false false))

(fn `DestroyActor`)

(fn `DestryBullet`)

(fn `EventHitCharacter`
  (params (Actor :type "Actor Object Reference")))

(fn `Firework`
  (`NiagaraFunctionLibrary.SpawnSystemAtLocation` "/Game/CoinGame/Good.Good" (`SceneComponent.K2_GetComponentLocation` (`self.Sphere`)))
  (`self.K2_DestroyActor`))

(fn `ParticlePosition`
  (`SceneComponent.K2_SetWorldTransform` (`self.Particle`) (`self.GetTransform`) false false))

(fn `UserConstructionScript`)

(fn `VRotation`)