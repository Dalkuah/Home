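; Enemy AI character that initializes with given HP and damage plus random size and tint, then fights the player.
; It attacks with size-scaled melee sphere traces, repeatable on a timer, or fireballs, and exposes blackboard target and walk-speed helpers.
; Incoming hits trigger knockback and a brief damage cooldown; death ragdolls it, spawns EXP and notifies its owner.
; Fast looping timers refresh a camera-facing name-tag HP widget; the sighting handler is disconnected.
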(event `TG_Attack`
  (if (not (`self.Dead`))
    (bind _returnvalue (`KismetSystemLibrary.K2_SetTimerDelegate` (delegate `Attack`) 0.01 true))
    (set `self.AT?` _returnvalue)))

(event `Attack`
  (bind _returnvalue (`self.K2_GetActorLocation`))
  (bind _size (`self.Size`))
  (if (not (`self.Dead`))
    (bind _outhits (`KismetSystemLibrary.SphereTraceMultiForObjects` _returnvalue (+ _returnvalue (* (`KismetMathLibrary.GetForwardVector` (`self.K2_GetActorRotation`)) (* _size 230.0))) (* _size 100.0) (`|MakeArray` "ObjectTypeQuery3" :!type "EObjectTypeQuery Enum")))
    (for _array_element _outhits
      (bind _asbp_player_ox (cast `/Game/aaaaa/ThirdPerson/Blueprints/BP_PlayerOX` (`.HitActor` (`GameplayStatics.BreakHitResult` _array_element))))
      (if (<= (`/Game/aaaaa/ThirdPerson/Blueprints/BP_PlayerOX.DamageDelay` _asbp_player_ox) 0.0)
        (bind _asbp_player_state (cast `/Game/CoinGame/GameMode/BP_PlayerState` (`Pawn.PlayerState` _asbp_player_ox)))
        (`self.AttackPlayer2`)
        (bind _followcamera (`/Game/aaaaa/ThirdPerson/Blueprints/BP_PlayerOX.FollowCamera` _asbp_player_ox))
        (`/Engine/EditorBlueprintResources/StandardMacros.IsValid` _followcamera
          (:`Is Valid`
            (`GameplayStatics.PlayWorldCameraShake` "/Game/CoinGame/BP_CameraShake.BP_CameraShake_C" (`SceneComponent.K2_GetComponentLocation` _followcamera) 0.0 500.0)))))))

(event `AttackPlayer2`
  (bind _returnvalue_location (`KismetMathLibrary.BreakTransform` (`self.GetTransform` (stale `Attack` _asbp_player_ox))))
  (`NiagaraFunctionLibrary.SpawnSystemAttached` "/Game/CoinGame/BloodFx_2.BloodFx_2" (`Character.Mesh` (stale `Attack` _asbp_player_ox)) "head" _returnvalue_location (struct) "KeepWorldPosition" true)
  (`/Game/CoinGame/GameMode/BP_PlayerState.AddDamage` (stale `Attack` _asbp_player_state) (`self.Damage`))
  (`self.LaunchCharacter` (stale `Attack` _asbp_player_ox) (* (`SceneComponent.GetForwardVector` (`self.Arrow1`)) 1000.0) false false)
  (set `/Game/aaaaa/ThirdPerson/Blueprints/BP_PlayerOX.DamageDelay` 0.5 (stale `Attack` _asbp_player_ox)))

(event `/Game/CoinGame/AISet.AISET`
  (params (EntityHP :type "Float (double-precision)") (EntityDamage :type "Float (double-precision)"))
  (bind _mesh (`self.Mesh`))
  (bind _size (`self.Size`))
  (bind _output_get (set `self.MaxHP` EntityHP))
  (set `self.HP` _output_get)
  (set `self.Damage` EntityDamage)
  (bind _output_get_2 (set `self.Size` (`KismetMathLibrary.RandomFloatInRange` 0.5 2.0)))
  (`self.SetActorScale3D` (`KismetMathLibrary.Conv_DoubleToVector` _output_get_2))
  (set `self.CloseDistance` (* _size 250.0))
  (set `self.LongDistance` (* _size 700.0))
  (bind _returnvalue (`PrimitiveComponent.CreateDynamicMaterialInstance` _mesh 0 "/Game/FourEvilDragonsHP/Materials/DragonTheSoulEater/GreenMat_Inst.GreenMat_Inst" "None"))
  (`MaterialInstanceDynamic.SetVectorParameterValue` _returnvalue "Variation" (`KismetMathLibrary.Conv_VectorToLinearColor` (`KismetMathLibrary.RandomUnitVector`)))
  (`PrimitiveComponent.SetMaterial` _mesh 0 _returnvalue))

(event `Stop_TG_Attack`
  (`KismetSystemLibrary.K2_ClearAndInvalidateTimerHandle` (`self.AT?`)))

(event `Attack Player`
  (bind _returnvalue (`self.K2_GetActorLocation`))
  (bind _size (`self.Size`))
  (if (not (`self.Dead`))
    (bind (_outhits _returnvalue_2) (`KismetSystemLibrary.SphereTraceMultiForObjects` _returnvalue (+ _returnvalue (* (`KismetMathLibrary.GetForwardVector` (`self.K2_GetActorRotation`)) (* _size 250.0))) (* _size 100.0) (`|MakeArray` "ObjectTypeQuery3" :!type "EObjectTypeQuery Enum")))
    (for _array_element _outhits
      (if _returnvalue_2
        (bind _asbp_player_ox (cast `/Game/aaaaa/ThirdPerson/Blueprints/BP_PlayerOX` (`.HitActor` (`GameplayStatics.BreakHitResult` _array_element))))
        (cast `/Game/CoinGame/GameMode/BP_PlayerState` (`Pawn.PlayerState` _asbp_player_ox))
        (`|PlayMontage` (`self.Mesh`) "/Game/FourEvilDragonsHP/Animations/DragonTheSoulEater/AttackMouthAnim_Montage.AttackMouthAnim_Montage")))))

(event `self.ReceiveBeginPlay`
  (bind _size (`self.Size`))
  (`KismetSystemLibrary.K2_SetTimer` null "SetProgressHP" 0.01 true)
  (`KismetSystemLibrary.K2_SetTimer` null "UpdateTag" 0.01 true)
  (`NiagaraFunctionLibrary.SpawnSystemAtLocation` "/Game/MyGame/AI/SpawnParticle.SpawnParticle" (`SceneComponent.K2_GetComponentLocation` (`self.Mesh`)) (struct) (3.0 3.0 3.0))
  (set `self.CloseDistance` (* _size 250.0))
  (set `self.LongDistance` (* _size 700.0)))

(event `self.PawnSensing.OnSeePawn`
  (params (Pawn :type "Pawn Object Reference")))

(event `OnFly`
  (bind _charactermovement (`self.CharacterMovement`))
  (`CharacterMovementComponent.SetMovementMode` _charactermovement "MOVE_Flying" 0)
  (set `CharacterMovementComponent.bOrientRotationToMovement` true _charactermovement))

(event `Attack2`
  (if (not (`self.Dead`))
    (`self.PlayAnimMontage` "/Game/FourEvilDragonsHP/Animations/DragonTheSoulEater/FlyAttackAnim_Montage.FlyAttackAnim_Montage")
    (`KismetSystemLibrary.Delay` 0.3)
    (if (`KismetMathLibrary.RandomBool`)
      (for _ (range 5)
        (`|SpawnActorFromClass` "/Game/CoinGame/BP_SmallFball1.BP_SmallFball1_C" (`KismetMathLibrary.MakeTransform` (`SceneComponent.GetSocketLocation` (`self.Mesh`) "Jaw") (`KismetMathLibrary.FindLookAtRotation` (`self.K2_GetActorLocation`) (`self.K2_GetActorLocation` (`GameplayStatics.GetPlayerCharacter` 0))) (`KismetMathLibrary.Conv_DoubleToVector` (* (`self.Size`) 0.3))) "Undefined" "OverrideRootScale" null null))
      (else
        (`|SpawnActorFromClass` "/Game/CoinGame/BP_Fball.BP_Fball_C" (`KismetMathLibrary.MakeTransform` (`SceneComponent.GetSocketLocation` (`self.Mesh`) "Jaw") (`KismetMathLibrary.FindLookAtRotation` (`self.K2_GetActorLocation`) (`self.K2_GetActorLocation` (`GameplayStatics.GetPlayerCharacter` 0))) (`KismetMathLibrary.Conv_DoubleToVector` (`self.Size`))) "Undefined" "OverrideRootScale" null null)))))

(event `Hit`
  (set `self.DamageDelay` 0.5)
  (`|PlayMontage` (`self.Mesh`) "/Game/FourEvilDragonsHP/Animations/DragonTheSoulEater/GetHitAnim_Montage.GetHitAnim_Montage"
    (:`OnCompleted`
      _)
    (:`OnInterrupted`
      _))
  (`self.Move`))

(event `NMove`)

(event `self.ReceiveTick`
  (params (DeltaSeconds :type "Float (single-precision)"))
  (bind _damagedelay (`self.DamageDelay`))
  (if (> _damagedelay 0.0)
    (set `self.DamageDelay` (- _damagedelay DeltaSeconds))
    (if (`NavMovementComponent.IsMovingOnGround` (`self.CharacterMovement`))
      (`self.LaunchCharacter` (0.0 0.0 30.0)))))

(event `Move`
  (`ActorComponent.SetActive` (`self.CharacterMovement`) true false))

(event `/Game/MyGame/AI/IF_Attack.Attack_ttt`
  (params (Attack_tt_S :type "/Game/MyGame/AI/ST_Attack Structure"))
  (bind _returnvalue_location (`KismetMathLibrary.BreakTransform` (`self.GetTransform`)))
  (if (`self.Dead`)
    _
    (elif (<= (`self.DamageDelay`) 0.0)
      (`self.AddDamage` Attack_tt_S_Damage_2_B762F29B490132550BCACF89D98709F7)
      (`self.LaunchCharacter` (`KismetMathLibrary.ClampVectorSize` (* (`KismetMathLibrary.GetForwardVector` (`KismetMathLibrary.FindLookAtRotation` (`self.K2_GetActorLocation` Attack_tt_S_Self_8_687AB4694E7CE9DCD425E1B14915CF34) (`self.K2_GetActorLocation`))) (* Attack_tt_S_Damage_2_B762F29B490132550BCACF89D98709F7 (`self.Knockback`))) 0.0 1000.0))
      (`NiagaraFunctionLibrary.SpawnSystemAttached` "/Game/CoinGame/BloodFx_2.BloodFx_2" (`self.Mesh`) "head" _returnvalue_location (struct) "KeepWorldPosition" true))))

(event `/Game/MyGame/Hook/ChainSelect.ChainDead?`
  (params (`ChainDead?` :type "Actor Object Reference") (seflC :type "Actor Object Reference"))
  (`/Engine/EditorBlueprintResources/StandardMacros.IsValid` seflC
    (:`Is Valid`
      (if (`self.Dead`)
        (message `/Game/MyGame/Hook/ChainSelect.ChainDead` seflC `ChainDead?`)))))

(event `Dead!`
  (`KismetSystemLibrary.Delay` 2.0)
  (`self.K2_DestroyActor`))

(event `/Game/MyGame/AI/AttackOK.OK!`
  (params (Type :type "/Game/MyGame/AI/ST_Attack Structure"))
  (if (`self.Dead`)
    _
    (elif (<= (`self.DamageDelay`) 0.0)
      (message `/Game/MyGame/AI/AttackOK.AttackOK` Type_Self_8_687AB4694E7CE9DCD425E1B14915CF34 true (make `/Game/MyGame/AI/ST_Attack` Type_Damage_2_B762F29B490132550BCACF89D98709F7 Type_Self_8_687AB4694E7CE9DCD425E1B14915CF34 Type_AttackType_15_4AB1FC5D42BD6FC82287CD87F2791D80 Type_Target_20_3CB942D44E55EF86AFC286A97DD84878)))))

(event `/Game/MyGame/AI/AttackOK.ChainSelectOK?`
  (params (Player :type "Actor Object Reference"))
  (if (`self.Dead`)
    _
    (elif (<= (`self.DamageDelay`) 0.0)
      (message `/Game/MyGame/AI/AttackOK.ChainSelectOK!` Player true self))))

(fn `AddDamage`
  (params (Damage :type "Float (double-precision)"))
  (bind (_returnvalue_roll _returnvalue_pitch _returnvalue_yaw) (`KismetMathLibrary.BreakRotator` (`self.K2_GetActorRotation`)))
  (`|ExecutionSequence`
    (:`then_0`
      (bind _output_get (set `self.HP` (- (`self.HP`) Damage)))
      (if (<= _output_get 0.0)
        (`self.Death`)
        (set `self.DamageDelay` 0.5)
        (else
          (`self.Hit`)
          (`self.K2_SetActorRotation` (`KismetMathLibrary.MakeRotator` 0.0 0.0 _returnvalue_yaw))
          (set `self.DamageDelay` 0.5))))))

(fn `ClearTarget`
  (`BlackboardComponent.ClearValue` (`AIBlueprintHelperLibrary.GetBlackboard` (`AIBlueprintHelperLibrary.GetAIController` self)) "Target"))

(fn `Death`
  (`PrimitiveComponent.SetSimulatePhysics` (`self.Mesh`) true)
  (`CharacterMovementComponent.DisableMovement` (`self.CharacterMovement`))
  (`PrimitiveComponent.SetCollisionEnabled` (`self.CapsuleComponent`) "NoCollision")
  (set `self.Dead` true)
  (`self.Dead!`)
  (for _ (range 1 2)
    (bind _returnvalue (`|SpawnActorFromClass` "/Game/CoinGame/Game/BP_EXP.BP_EXP_C" (`KismetMathLibrary.MakeTransform` (`self.K2_GetActorLocation`)) "Undefined" "OverrideRootScale" null null))
    (`/Engine/EditorBlueprintResources/StandardMacros.IsValid` _returnvalue
      (:`Is Valid`
        (message `/Game/CoinGame/Game/EntityEXP.!!EXP` _returnvalue 10)
        (message `/Game/CoinGame/AISet.EntityDEAD` (`self.GetOwner`) self)))))

(fn `GetTarget`
  (returns (Target :type "Actor Object Reference"))
  (return (cast `Actor` (`BlackboardComponent.GetValueAsObject` (`AIBlueprintHelperLibrary.GetBlackboard` (`AIBlueprintHelperLibrary.GetAIController` self)) "Target") :!pure true)))

(fn `SetProgressHP`
  (bind _maxhp (`self.MaxHP`))
  (bind `_as뚜샤쇼_name_tag_widget` (cast `/Game/CoinGame/뚜샤쇼_NameTag_Widget` (`WidgetComponent.GetUserWidgetObject` (`self.Widget`))))
  (`/Game/CoinGame/뚜샤쇼_NameTag_Widget.SetProgressHP` `_as뚜샤쇼_name_tag_widget` (`self.HP`) _maxhp (`KismetMathLibrary.FFloor` (/ _maxhp 60.0)) (`self.Name`)))

(fn `SetTarget`
  (params (NewTarget :type "Actor Object Reference"))
  (`BlackboardComponent.SetValueAsObject` (`AIBlueprintHelperLibrary.GetBlackboard` (`AIBlueprintHelperLibrary.GetAIController` self)) "Target" NewTarget))

(fn `UpdateTag`
  (bind _widget (`self.Widget`))
  (`SceneComponent.K2_SetWorldRotation` _widget (`KismetMathLibrary.FindLookAtRotation` (`SceneComponent.K2_GetComponentLocation` _widget) (`self.K2_GetActorLocation` (`GameplayStatics.GetPlayerCameraManager` 0))) false false))

(fn `UpdateWalkSpeed`
  (params (NewWalkSpeed :type "Float (double-precision)"))
  (set `CharacterMovementComponent.MaxWalkSpeed` NewWalkSpeed (`self.CharacterMovement`)))

(fn `UserConstructionScript`)