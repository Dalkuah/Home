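; Boss enemy character with a health nametag that faces the camera, mouth melee and fireball attacks, and ragdoll death.
; PawnSensing sets a blackboard flag on seeing the player and jumps if the player is far away.
; AttackPlayer plays the bite montage when in range, while a toggleable timer repeats sphere traces that damage and launch players.
; Incoming hits reduce HP, with attack events adding knockback, blood and a damage cooldown.
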(event `self.ReceiveAnyDamage`
  (params (Damage :type "Float (single-precision)") (DamageType :type "DamageType Object Reference") (InstigatedBy :type "Controller Object Reference") (DamageCauser :type "Actor Object Reference"))
  (bind (_returnvalue_roll _returnvalue_pitch _returnvalue_yaw) (`KismetMathLibrary.BreakRotator` (`self.K2_GetActorRotation`)))
  (bind _output_get (set `self.HP` (- (`self.HP`) Damage)))
  (if (<= _output_get 0.0)
    (`self.Death`)
    (else
      (`self.PlayAnimMontage` "/Game/FourEvilDragonsHP/Animations/DragonTheSoulEater/GetHitAnim_Montage.GetHitAnim_Montage")
      (`self.K2_SetActorRotation` (`KismetMathLibrary.MakeRotator` 0.0 0.0 _returnvalue_yaw)))))

(event `TG_Attack`
  (bind _returnvalue (`KismetSystemLibrary.K2_SetTimerDelegate` (delegate `Attack`) 0.01 true))
  (set `self.AT?` _returnvalue))

(event `self.ReceiveBeginPlay`
  (`KismetSystemLibrary.K2_SetTimer` null "SetProgressHP" 0.01 true)
  (`KismetSystemLibrary.K2_SetTimer` null "UpdateTag" 0.01 true)
  (`NiagaraFunctionLibrary.SpawnSystemAtLocation` "/Game/MyGame/AI/SpawnParticle.SpawnParticle" (`SceneComponent.K2_GetComponentLocation` (`self.Mesh`)) (struct) (3.0 3.0 3.0)))

(event `Attack`
  (bind _returnvalue (`self.K2_GetActorLocation`))
  (bind _outhits (`KismetSystemLibrary.SphereTraceMultiForObjects` _returnvalue (+ _returnvalue (* (`KismetMathLibrary.GetForwardVector` (`self.K2_GetActorRotation`)) 250.0)) 100.0 (`|MakeArray` "ObjectTypeQuery3" :!type "EObjectTypeQuery Enum")))
  (for _array_element _outhits
    (bind _asbp_player_ox (cast `/Game/aaaaa/ThirdPerson/Blueprints/BP_PlayerOX` (`.HitActor` (`GameplayStatics.BreakHitResult` _array_element))))
    (if (<= (`/Game/aaaaa/ThirdPerson/Blueprints/BP_PlayerOX.DamageDelay` _asbp_player_ox) 0.0)
      (bind _asbp_player_state (cast `/Game/CoinGame/GameMode/BP_PlayerState` (`Pawn.PlayerState` _asbp_player_ox)))
      (`self.AttackPlayer2`)
      (bind _followcamera (`/Game/aaaaa/ThirdPerson/Blueprints/BP_PlayerOX.FollowCamera` _asbp_player_ox))
      (`/Engine/EditorBlueprintResources/StandardMacros.IsValid` _followcamera
        (:`Is Valid`
          (`GameplayStatics.PlayWorldCameraShake` "/Game/CoinGame/BP_CameraShake.BP_CameraShake_C" (`SceneComponent.K2_GetComponentLocation` _followcamera) 0.0 500.0))))))

(event `AttackPlayer2`
  (bind _returnvalue_location (`KismetMathLibrary.BreakTransform` (`self.GetTransform` (stale `Attack` _asbp_player_ox))))
  (`NiagaraFunctionLibrary.SpawnSystemAttached` "/Game/CoinGame/BloodFx_2.BloodFx_2" (`Character.Mesh` (stale `Attack` _asbp_player_ox)) "head" _returnvalue_location (struct) "KeepWorldPosition" true)
  (`/Game/CoinGame/GameMode/BP_PlayerState.AddDamage` (stale `Attack` _asbp_player_state) 30.0)
  (`self.LaunchCharacter` (stale `Attack` _asbp_player_ox) (* (`SceneComponent.GetForwardVector` (`self.Arrow1`)) 3000.0) false false)
  (set `/Game/aaaaa/ThirdPerson/Blueprints/BP_PlayerOX.DamageDelay` 0.5 (stale `Attack` _asbp_player_ox)))

(event `self.PawnSensing.OnSeePawn`
  (params (Pawn :type "Pawn Object Reference"))
  (if (not (`self.Dead`))
    (bind _asbp_player_ox (cast `/Game/aaaaa/ThirdPerson/Blueprints/BP_PlayerOX` Pawn))
    (`BlackboardComponent.SetValueAsBool` (`AIBlueprintHelperLibrary.GetBlackboard` (`AIBlueprintHelperLibrary.GetAIController` self)) "HasSeenPlayer?" true)
    (if (>= (`KismetMathLibrary.Vector_Distance` (`self.K2_GetActorLocation` _asbp_player_ox) (`self.K2_GetActorLocation`)) 1000.0)
      (`self.Jump`))))

(event `Stop_TG_Attack`
  (`KismetSystemLibrary.K2_ClearAndInvalidateTimerHandle` (`self.AT?`)))

(event `Attack Player`
  (bind _returnvalue (`self.K2_GetActorLocation`))
  (if (not (`self.Dead`))
    (bind (_outhits _returnvalue_2) (`KismetSystemLibrary.SphereTraceMultiForObjects` _returnvalue (+ _returnvalue (* (`KismetMathLibrary.GetForwardVector` (`self.K2_GetActorRotation`)) 250.0)) 100.0 (`|MakeArray` "ObjectTypeQuery3" :!type "EObjectTypeQuery Enum")))
    (for _array_element _outhits
      (if _returnvalue_2
        (bind _asbp_player_ox (cast `/Game/aaaaa/ThirdPerson/Blueprints/BP_PlayerOX` (`.HitActor` (`GameplayStatics.BreakHitResult` _array_element))))
        (cast `/Game/CoinGame/GameMode/BP_PlayerState` (`Pawn.PlayerState` _asbp_player_ox))
        (`|PlayMontage` (`self.Mesh`) "/Game/FourEvilDragonsHP/Animations/DragonTheSoulEater/AttackMouthAnim_Montage.AttackMouthAnim_Montage")))))

(event `Attack2`
  (bind (_returnvalue_location _returnvalue_rotation) (`KismetMathLibrary.BreakTransform` (`self.GetTransform`)))
  (if (not (`self.Dead`))
    (`self.PlayAnimMontage` "/Game/FourEvilDragonsHP/Animations/DragonTheSoulEater/FlyAttackAnim_Montage.FlyAttackAnim_Montage")
    (`|SpawnActorFromClass` "/Game/CoinGame/BP_Fball.BP_Fball_C" (`KismetMathLibrary.MakeTransform` (`SceneComponent.GetSocketLocation` (`self.Mesh`) "Jaw") _returnvalue_rotation) "Undefined" "OverrideRootScale" null null)))

(event `self.ReceiveTick`
  (params (DeltaSeconds :type "Float (single-precision)"))
  (bind _damagedelay (`self.DamageDelay`))
  (if (> _damagedelay 0.0)
    (set `self.DamageDelay` (- _damagedelay DeltaSeconds))))

(event `/Game/MyGame/AI/IF_Attack.Attack_ttt`
  (params (IF_ATTACK_S :type "/Game/MyGame/AI/ST_Attack Structure"))
  (bind _returnvalue_location (`KismetMathLibrary.BreakTransform` (`self.GetTransform`)))
  (if (<= (`self.DamageDelay`) 0.0)
    (`self.AddDamage` IF_ATTACK_S_Damage_2_B762F29B490132550BCACF89D98709F7)
    (`self.LaunchCharacter` (* (`KismetMathLibrary.GetForwardVector` (`KismetMathLibrary.FindLookAtRotation` (`self.K2_GetActorLocation` IF_ATTACK_S_Self_8_687AB4694E7CE9DCD425E1B14915CF34) (`self.K2_GetActorLocation`))) (* IF_ATTACK_S_Damage_2_B762F29B490132550BCACF89D98709F7 50.0)))
    (`NiagaraFunctionLibrary.SpawnSystemAttached` "/Game/CoinGame/BloodFx_2.BloodFx_2" (`self.Mesh`) "head" _returnvalue_location (struct) "KeepWorldPosition" true)))

(event `/Game/MyGame/AI/AttackOK.OK!`
  (params (Actor :type "Actor Object Reference"))
  (if (<= (`self.DamageDelay`) 0.0)
    (message `/Game/MyGame/AI/AttackOK.AttackOK` Actor true self)))

(fn `AddDamage`
  (params (Damage :type "Float (double-precision)"))
  (bind (_returnvalue_roll _returnvalue_pitch _returnvalue_yaw) (`KismetMathLibrary.BreakRotator` (`self.K2_GetActorRotation`)))
  (bind _output_get (set `self.HP` (- (`self.HP`) Damage)))
  (if (<= _output_get 0.0)
    (`self.Death`)
    (else
      (`self.PlayAnimMontage` "/Game/FourEvilDragonsHP/Animations/DragonTheSoulEater/GetHitAnim_Montage.GetHitAnim_Montage")
      (`self.K2_SetActorRotation` (`KismetMathLibrary.MakeRotator` 0.0 0.0 _returnvalue_yaw))
      (set `self.DamageDelay` 0.5))))

(fn `Death`
  (`PrimitiveComponent.SetSimulatePhysics` (`self.Mesh`) true)
  (`CharacterMovementComponent.DisableMovement` (`self.CharacterMovement`))
  (`PrimitiveComponent.SetCollisionEnabled` (`self.CapsuleComponent`) "NoCollision")
  (set `self.Dead` true))

(fn `SetProgressHP`
  (bind `_as뚜샤쇼_name_tag_widget` (cast `/Game/CoinGame/뚜샤쇼_NameTag_Widget` (`WidgetComponent.GetUserWidgetObject` (`self.Widget`))))
  (`/Game/CoinGame/뚜샤쇼_NameTag_Widget.SetProgressHP` `_as뚜샤쇼_name_tag_widget` (`self.HP`) (`self.MaxHP`)))

(fn `UpdateTag`
  (bind _widget (`self.Widget`))
  (`SceneComponent.K2_SetWorldRotation` _widget (`KismetMathLibrary.FindLookAtRotation` (`SceneComponent.K2_GetComponentLocation` _widget) (`self.K2_GetActorLocation` (`GameplayStatics.GetPlayerCameraManager` 0))) false false))

(fn `UserConstructionScript`)